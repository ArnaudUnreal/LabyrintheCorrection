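; BP_Piege is a labyrinth trap that kills the player when the first-person character overlaps its trigger sphere.
; The overlap slides the static mesh along X, then after a short delay adds a W_Blood widget to the viewport.
; It also removes the IMC_Moves input mapping to block player input while a timeline tints the blood image.
; When the timeline finishes, the game quits after a brief pause.
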(event OnComponentBeginOverlap(Sphere)
  (params (OverlappedComponent :type Primitive%20Component%20Object%20Reference) (OtherActor :type Actor%20Object%20Reference) (OtherComp :type Primitive%20Component%20Object%20Reference) (OtherBodyIndex :type Integer) (bFromSweep :type Boolean) (SweepResult :type Hit%20Result%20Structure%20%28by%20ref%29))
  (Utilities|Casting|CastToBP_FirstPersonCharacter OtherActor)
  (Components|MoveComponentTo (Variables|Default|GetStaticMesh) "700.000000,0.000000,0.000000" "0, 0, 0" false false 0.2 false)
  ;[1 1 1] Bonus
  (Utilities|FlowControl|Delay 0.5)
  (bind _aspc_labyrinthe (Utilities|Casting|CastToPC_Labyrinthe (Game|GetPlayerController 0)))
  (bind _returnvalue (UserInterface|CreateWidget "/Game/Le_Labyrinthe/UMG/W_Blood.W_Blood_C" _aspc_labyrinthe))
  (Variables|Default|SetImage%2026 (Variables|/Game/Le_Labyrinthe/UMG/W_Blood.W_Blood_C|GetImage_26 _returnvalue))
  (UserInterface|Viewport|AddtoViewport _returnvalue 0)
  (Utilities|IsValid (PlayerController|LocalPlayerSubsystems|GetEnhancedInputLocalPlayerSubsystem _aspc_labyrinthe)
    (:Is%20Valid
      (Input|RemoveMappingContext (PlayerController|LocalPlayerSubsystems|GetEnhancedInputLocalPlayerSubsystem _aspc_labyrinthe) "/Game/Le_Labyrinthe/Inputs/IMC_Moves.IMC_Moves" "(bIgnoreAllPressedKeysUntilRelease=True,bForceImmediately=False)")
      (bind _color (Timeline|Timeline PlayFromStart)
        (:Update
          (Class|Image|SetBrushTintColor (Variables|Default|GetImage%2026) (Utilities|Struct|MakeSlateColor _color "UseColor_Specified")))
        (:Finished
          (Utilities|FlowControl|Delay 0.2)
          (Game|QuitGame 0 "Quit" false))))))

(fn ConstructionScript
  (|CallParentFunction))