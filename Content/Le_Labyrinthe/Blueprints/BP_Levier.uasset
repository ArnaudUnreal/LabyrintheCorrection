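; BP_Levier is a lever in the labyrinth that locks and unlocks a secret passage.
; Each eventActivate flips IsActivated and plays a Timeline forward or in reverse, rotating the lever between its start pose and a pitched-down pose.
; The Timeline track feeds RInterpTo's DeltaTime input.
; When the Timeline finishes, it writes the state to GI_Labyrinthe.Unlocked, prints it and calls EventCheckOpening.
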(event Custom|eventActivate
  (bind _isa (Utilities|FlowControl|FlipFlop)
    (:A
      (Variables|Default|SetIsActivated _isa)
      (bind _newtrack_0 (Timeline|Timeline PlayFromStart)
        (:Update
          (Transformation|SetRelativeRotation (Variables|Default|Getlevier) (Math|Interpolation|RInterpTo (Variables|Default|GetStart%20Rotation%20Levier) (Variables|Default|GetEnf%20Rotation%20Levier) _newtrack_0 0.0) false false))
        (:Finished
          (bind _asgi_labyrinthe (Utilities|Casting|CastToGI_Labyrinthe (Game|GetGameInstance)))
          (bind _output_get (Variables|/Game/Le_Labyrinthe/Blueprints/Game/GI_Labyrinthe.GI_Labyrinthe_C|SetUnlocked _asgi_labyrinthe (Variables|Default|GetIsActivated)))
          (Development|PrintString (Utilities|String|Append "Etat UNLOCKED Passage secret : " (Utilities|String|ToString(Boolean) _output_get)))
          (Default|EventCheckOpening _asgi_labyrinthe))))
    (:B
      (Variables|Default|SetIsActivated _isa)
      (Timeline|Timeline ReverseFromEnd))))

(event EventBeginPlay
  (bind _output_get (Variables|Default|SetStart%20Rotation%20Levier (Variables|/Script/Engine.SceneComponent|GetRelativeRotation (Variables|Default|Getlevier))))
  (Variables|Default|SetEnf%20Rotation%20Levier (Math|Rotator|MakeRotator (.Roll (Math|Rotator|BreakRotator _output_get)) (+ (.Pitch (Math|Rotator|BreakRotator _output_get)) -9e+01) (.Yaw (Math|Rotator|BreakRotator _output_get)))))

(fn ConstructionScript)